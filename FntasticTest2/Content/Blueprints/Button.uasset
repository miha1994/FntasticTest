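; Clickable 2D button actor that tells its referenced Nest to make a turtle.
; On BeginPlay it enables click events, mouse-over events and the cursor on the first player controller, then shows the idle sprite.
; Clicking its PaperSprite switches to the pressed sprite and calls MakeTurtle on the Nest.
; Releasing the mouse or moving the cursor off restores the idle sprite.
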(event OnEndCursorOver(PaperSprite)
  (params (TouchedComponent :type Primitive%20Component%20Object%20Reference))
  (CallFunction|SetIdle))

(event OnClicked(PaperSprite)
  (params (TouchedComponent :type Primitive%20Component%20Object%20Reference) (ButtonPressed :type Key%20Structure :default "None"))
  (CallFunction|MakeTurtle))

(event OnReleased(PaperSprite)
  (params (TouchedComponent :type Primitive%20Component%20Object%20Reference) (ButtonReleased :type Key%20Structure :default "None"))
  (CallFunction|SetIdle))

(event Custom|Make%20Turtle
  (Rendering|Components|Sprite|SetSprite (Variables|Default|GetPaperSprite) (Variables|Default|Getsprite_pressed))
  (Default|MakeTurtle (Variables|Default|Getnest)))

(event Custom|Set%20Idle
  (Rendering|Components|Sprite|SetSprite (Variables|Default|GetPaperSprite) (Variables|Default|Getsprite_idle)))

(event EventBeginPlay
  (bind _returnvalue (Game|GetPlayerController 0))
  (Variables|/Script/Engine.PlayerController|SetbEnableClickEvents _returnvalue true)
  (Variables|/Script/Engine.PlayerController|SetbEnableMouseOverEvents _returnvalue true)
  (Variables|/Script/Engine.PlayerController|SetbShowMouseCursor _returnvalue true)
  (CallFunction|SetIdle))

(event EventTick
  (params (DeltaSeconds :type Float%20%28single-precision%29)))

(fn ConstructionScript)