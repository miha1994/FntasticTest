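; Short-lived sprite particle actor that bursts out, falls and shrinks away.
; On BeginPlay it picks a random lifetime and an upward-biased random velocity confined to the XZ plane.
; Tick moves the root without sweeping, adds manual downward acceleration and scales the sprite by the remaining lifetime fraction, destroying the actor when time runs out.
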(event EventBeginPlay
  (bind _returnvalue (Math|Random|RandomUnitVector))
  (bind _returnvalue_2 (+ _returnvalue "0.000000,0.000000,1.000000"))
  (bind (_x _y _z) (Math|Vector|BreakVector _returnvalue_2))
  (bind _output_get (Variables|Default|Setmax_time (Math|Random|RandomFloatinRange 0.4 1.2)))
  (Variables|Default|Settime _output_get)
  (Variables|Default|Setvelocity (* (Math|Vector|MakeVector _x 0.0 _z) 4e+01)))

(event Collision|EventActorBeginOverlap
  (params (OtherActor :type Actor%20Object%20Reference)))

(event EventTick
  (params (DeltaSeconds :type Float%20%28single-precision%29))
  (Transformation|AddRelativeLocation (Variables|Default|GetDefaultSceneRoot) (* DeltaSeconds (Variables|Default|Getvelocity)) false false)
  (Variables|Default|Setvelocity (+ (* (Math|Vector|VectorDown) DeltaSeconds 2e+02) (Variables|Default|Getvelocity)))
  (Transformation|SetWorldScale3D (Variables|Default|GetSprite) (* (Class|KismetMathLibrary|VectorOne) (/ (- (Variables|Default|Gettime) DeltaSeconds) (Variables|Default|Getmax_time))))
  (bind _output_get (Variables|Default|Settime (- (Variables|Default|Gettime) DeltaSeconds)))
  (if (< _output_get 0.0)
    (Actor|DestroyActor)))

(fn ConstructionScript)