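; Turtle actor that walks toward a goal nest, set along with its type through Init, and destroys itself on arrival.
; Tick alternates a full-speed phase with a shorter phase whose type-based speed scale keeps it walking, pauses it with an idle flipbook, or backs it up.
; The sprite flips with horizontal movement, while timers emit step sounds and particles.
; Spawning and arrival each play a cue and a particle burst.
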(event Custom|Update%20State
  (bind _sprite (Variables|Default|GetSprite))
  (if (Math|Conversions|ToBoolean(Integer) (Variables|Default|Getstate))
    (Variables|Default|Settime 1.0)
    (else
      (Variables|Default|Settime 0.5)))
  (if (== (Variables|Default|Getstate1_scale) 0.0)
    (if (Math|Conversions|ToBoolean(Integer) (Variables|Default|Getstate))
      (Sprite|SetFlipbook _sprite "/Game/Sprites/FB_hero_walk.FB_hero_walk")
      (else
        (Sprite|SetFlipbook _sprite "/Game/Sprites/FB_hero_idle.FB_hero_idle"))))
  (Variables|Default|Setstate (- 1 (Variables|Default|Getstate))))

(event Custom|Spawn%20Particle
  (params (y_offset :type Float%20%28double-precision%29))
  (Game|SpawnActorfromClass "/Game/Blueprints/Particle.Particle_C" (Math|Conversions|ToTransform(Vector) (+ (Math|Vector|MakeVector 0.0 y_offset 0.0) (Transformation|GetActorLocation))) "AlwaysSpawn" 0 0))

(event Custom|Particle%20Time%20Update
  (params (Delta%20Seconds :type Float%20%28double-precision%29))
  (bind _output_get (Variables|Default|Setsound_time (- (Variables|Default|Getsound_time) Delta%20Seconds)))
  (Variables|Default|Setparticle_time (- (Variables|Default|Getparticle_time) Delta%20Seconds))
  (if (< (- (Variables|Default|Getparticle_time) Delta%20Seconds) 0.0)
    (Variables|Default|Setparticle_time (Math|Random|RandomFloatinRange 0.2 0.4))
    (CallFunction|SpawnParticle 1.0))
  (if (< _output_get 0.0)
    (Variables|Default|Setsound_time 0.3)
    (Audio|PlaySoundatLocation "/Game/Sounds/step_Cue.step_Cue" (Transformation|GetActorLocation) "0, 0, 0" 1.0 1.0 0.0 0 0 0 0)))

(event EventBeginPlay
  (Audio|PlaySoundatLocation "/Game/Sounds/enter_Cue.enter_Cue" (Transformation|GetActorLocation) "0, 0, 0" 1.0 1.0 0.0 0 0 0 0)
  (Variables|Default|Setsound_time 0.1)
  (Variables|Default|Setparticle_time (Math|Random|RandomFloatinRange 0.2 0.4))
  (Variables|Default|Setstate 0)
  (Variables|Default|Settime 1.0)
  (for _index (range 0 8)
    (CallFunction|SpawnParticle -1.0)))

(event Collision|EventActorBeginOverlap
  (params (OtherActor :type Actor%20Object%20Reference)))

(event EventTick
  (params (DeltaSeconds :type Float%20%28single-precision%29))
  (bind _returnvalue (Transformation|GetActorLocation))
  (bind _goal_nest (Variables|Default|Getgoal_nest))
  (bind _returnvalue_2 (Transformation|GetActorLocation _goal_nest))
  (bind _returnvalue_3 (- _returnvalue_2 _returnvalue))
  (switch int (Variables|Default|Getstate)
    (:0
      (Variables|Default|Setcurrent_scale 1.0))
    (:1
      (Variables|Default|Setcurrent_scale (Variables|Default|Getstate1_scale))))
  (bind _output_get (Variables|Default|Settime (- (Variables|Default|Gettime) DeltaSeconds)))
  (Transformation|AddRelativeLocation (Variables|Collision|GetCapsuleComponent) (* DeltaSeconds 5e+01 (Variables|Default|Getcurrent_scale) (Math|Vector|Normalize _returnvalue_3)) false false)
  (if (== (.X (Math|Vector|BreakVector (* DeltaSeconds 5e+01 (Variables|Default|Getcurrent_scale) (Math|Vector|Normalize _returnvalue_3)))) 0.0)
    _
    (else
      (CallFunction|ParticleTimeUpdate DeltaSeconds)
      (Transformation|SetWorldScale3D (Variables|Default|GetSprite) (+ (* (Math|Float|Sign(Float) (.X (Math|Vector|BreakVector (* DeltaSeconds 5e+01 (Variables|Default|Getcurrent_scale) (Math|Vector|Normalize _returnvalue_3))))) "1.000000,0.000000,0.000000") "0.000000,1.000000,1.000000"))))
  (if (< _output_get 0.0)
    (CallFunction|UpdateState))
  (if (< (Math|Vector|VectorLength _returnvalue_3) 1.0)
    (for _index (range 0 8)
      (CallFunction|SpawnParticle -1.0))
    (Audio|PlaySoundatLocation "/Game/Sounds/exit_Cue.exit_Cue" (Transformation|GetActorLocation) "0, 0, 0" 1.0 1.0 0.0 0 0 0 0)
    (Actor|DestroyActor)))

(fn ConstructionScript)

(fn Init
  (params (type :type Integer) (goal :type Nest%20Object%20Reference))
  (Variables|Default|Setgoal_nest goal)
  (bind _output_get (Variables|Default|Settype_id type))
  (switch int _output_get
    (:0
      (Variables|Default|Setstate1_scale 1.0 :!label _label))
    (:1
      (goto _label))
    (:2
      (Variables|Default|Setstate1_scale 0.0))
    (:3
      (Variables|Default|Setstate1_scale -1.0))))